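; AISpawnerOne is an AI spawner that creates AI_One pawns at random points inside its SpawnVolume box.
; While SpawnLimit is above zero, Tick calls SpawnEnemy every frame, and its one-second Delay throttles spawning to roughly one pawn per second.
; SpawnLimit is never decremented here, and SpawnerActive is set but never read.
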(event `self.ReceiveBeginPlay`
  (set `self.spawnerActive` true))

(event `self.ReceiveTick`
  (params (DeltaSeconds :type "Float (single-precision)"))
  (if (> (`self.spawnLimit`) 0)
    (`self.SpawnEnemy`)
    (else
      (set `self.spawnerActive` false))))

(event `SpawnEnemy`
  (bind _spawnvolume (`self.SpawnVolume`))
  (`KismetSystemLibrary.Delay` 1.0)
  (`AIBlueprintHelperLibrary.SpawnAIFromClass` "/Game/Blueprints/AI/AI_One.AI_One_C" null (`KismetMathLibrary.RandomPointInBoundingBox` (`SceneComponent.K2_GetComponentLocation` _spawnvolume) (`BoxComponent.GetScaledBoxExtent` _spawnvolume))))

(fn `UserConstructionScript`)