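; AI_Three_Shield is a shield Blueprint with four barriers that block projectiles of type ProjectileTypeOne.
; Each barrier collision component handles its own begin-overlap event, casts the overlapping actor to ProjectileTypeOne and destroys it on success.
; Other actors are ignored, and the construction script is empty.
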(event `self.BarrierOneCollision.OnComponentBeginOverlap`
  (params (OverlappedComponent :type "PrimitiveComponent Object Reference") (OtherActor :type "Actor Object Reference") (OtherComp :type "PrimitiveComponent Object Reference") (OtherBodyIndex :type Integer) (bFromSweep :type Boolean) (SweepResult :type "HitResult Structure (by ref)"))
  (bind _asprojectile_type_one (cast `/Game/Blueprints/ProjectileTypeOne` OtherActor))
  (`self.K2_DestroyActor` _asprojectile_type_one))

(event `self.BarrierTwoCollision.OnComponentBeginOverlap`
  (params (OverlappedComponent :type "PrimitiveComponent Object Reference") (OtherActor :type "Actor Object Reference") (OtherComp :type "PrimitiveComponent Object Reference") (OtherBodyIndex :type Integer) (bFromSweep :type Boolean) (SweepResult :type "HitResult Structure (by ref)"))
  (bind _asprojectile_type_one (cast `/Game/Blueprints/ProjectileTypeOne` OtherActor))
  (`self.K2_DestroyActor` _asprojectile_type_one))

(event `self.BarrierThreeCollision.OnComponentBeginOverlap`
  (params (OverlappedComponent :type "PrimitiveComponent Object Reference") (OtherActor :type "Actor Object Reference") (OtherComp :type "PrimitiveComponent Object Reference") (OtherBodyIndex :type Integer) (bFromSweep :type Boolean) (SweepResult :type "HitResult Structure (by ref)"))
  (bind _asprojectile_type_one (cast `/Game/Blueprints/ProjectileTypeOne` OtherActor))
  (`self.K2_DestroyActor` _asprojectile_type_one))

(event `self.BarrierFourCollision.OnComponentBeginOverlap`
  (params (OverlappedComponent :type "PrimitiveComponent Object Reference") (OtherActor :type "Actor Object Reference") (OtherComp :type "PrimitiveComponent Object Reference") (OtherBodyIndex :type Integer) (bFromSweep :type Boolean) (SweepResult :type "HitResult Structure (by ref)"))
  (bind _asprojectile_type_one (cast `/Game/Blueprints/ProjectileTypeOne` OtherActor))
  (`self.K2_DestroyActor` _asprojectile_type_one))

(fn `UserConstructionScript`)