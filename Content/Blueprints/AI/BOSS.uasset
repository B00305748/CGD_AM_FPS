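; Boss enemy that aims at the FPS player and fires projectiles while the player is inside its detection volume.
; Every Tick it looks up the FPSController and rotates the spawn point toward its Tracker.
; PlayerDetector overlaps toggle firing, with a Delay on Tick throttling BOSS_Projectile spawns to roughly one per second.
; ProjectileTypeOne hits on BossCollision subtract health and destroy the boss when it runs out.
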(event `self.ReceiveTick`
  (params (DeltaSeconds :type "Float (single-precision)"))
  (bind _projectilespawnpoint (`self.ProjectileSpawnPoint`))
  (bind _outactors (`GameplayStatics.GetAllActorsOfClass` "/Game/Blueprints/FPSController.FPSController_C"))
  (bind _asfpscontroller (cast `/Game/Blueprints/FPSController` (`|GetArrayItem` _outactors)))
  (`SceneComponent.K2_SetWorldRotation` (`self.ProjectileSpawnPoint`) (`KismetMathLibrary.FindLookAtRotation` (`SceneComponent.K2_GetComponentLocation` (`self.ProjectileSpawnPoint`)) (`SceneComponent.K2_GetComponentLocation` (`/Game/Blueprints/FPSController.Tracker` _asfpscontroller))) false false)
  (if (`self.playerDetected`)
    (`KismetSystemLibrary.Delay` 1.0)
    (`|SpawnActorFromClass` "/Game/Blueprints/AI/BOSS_Projectile.BOSS_Projectile_C" (`KismetMathLibrary.MakeTransform` (`SceneComponent.K2_GetComponentLocation` _projectilespawnpoint) (`SceneComponent.K2_GetComponentRotation` _projectilespawnpoint)) "Undefined" "OverrideRootScale" null null)))

(event `self.playerDetector.OnComponentBeginOverlap`
  (params (OverlappedComponent :type "PrimitiveComponent Object Reference") (OtherActor :type "Actor Object Reference") (OtherComp :type "PrimitiveComponent Object Reference") (OtherBodyIndex :type Integer) (bFromSweep :type Boolean) (SweepResult :type "HitResult Structure (by ref)"))
  (cast `/Game/Blueprints/FPSController` OtherActor)
  (set `self.playerDetected` true))

(event `self.playerDetector.OnComponentEndOverlap`
  (params (OverlappedComponent :type "PrimitiveComponent Object Reference") (OtherActor :type "Actor Object Reference") (OtherComp :type "PrimitiveComponent Object Reference") (OtherBodyIndex :type Integer))
  (cast `/Game/Blueprints/FPSController` OtherActor)
  (set `self.playerDetected` false))

(event `self.bossCollision.OnComponentBeginOverlap`
  (params (OverlappedComponent :type "PrimitiveComponent Object Reference") (OtherActor :type "Actor Object Reference") (OtherComp :type "PrimitiveComponent Object Reference") (OtherBodyIndex :type Integer) (bFromSweep :type Boolean) (SweepResult :type "HitResult Structure (by ref)"))
  (bind _asprojectile_type_one (cast `/Game/Blueprints/ProjectileTypeOne` OtherActor))
  (set `self.bossHealth` (- (`self.bossHealth`) (`/Game/Blueprints/ProjectileTypeOne.projectileDamageAgainstBoss` _asprojectile_type_one)))
  (if (not (> (`self.bossHealth`) 0.0))
    (`self.K2_DestroyActor`)))

(fn `UserConstructionScript`)