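; CORE_LevelThree is the level three destructible core, a target that jumps around inside a box zone.
; Tick feeds a Delay that periodically teleports the sphere child actor to a random point within CORETPZone.
; Overlaps from ProjectileTypeThree subtract the projectile's damage from AiHealth and play a hit sound.
; When health runs out, it sets UnlockedThree on the first FPSController found and destroys itself.
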(event `self.ReceiveTick`
  (params (DeltaSeconds :type "Float (single-precision)"))
  (bind _core_tp_zone (`self.CORE_TP_Zone`))
  (`KismetSystemLibrary.Delay` 2.0)
  (`SceneComponent.K2_SetWorldLocation` (`self.CORE_SphereChildActor`) (`KismetMathLibrary.RandomPointInBoundingBox` (`SceneComponent.K2_GetComponentLocation` _core_tp_zone) (`BoxComponent.GetScaledBoxExtent` _core_tp_zone)) false true))

(event `self.CORE_SphereChildActorCollision.OnComponentBeginOverlap`
  (params (OverlappedComponent :type "PrimitiveComponent Object Reference") (OtherActor :type "Actor Object Reference") (OtherComp :type "PrimitiveComponent Object Reference") (OtherBodyIndex :type Integer) (bFromSweep :type Boolean) (SweepResult :type "HitResult Structure (by ref)"))
  (bind _asprojectile_type_three (cast `/Game/Blueprints/ProjectileTypeThree` OtherActor))
  (bind _output_get (set `self.aiHealth` (- (`self.aiHealth`) (`/Game/Blueprints/ProjectileTypeThree.projectileDamageValue` _asprojectile_type_three))))
  (`GameplayStatics.PlaySoundAtLocation` "/Game/Sounds/corehit.corehit" (`SceneComponent.K2_GetComponentLocation` (`self.CORE_SphereChildActor`)) (struct) 1.0 1.0 0.0 null null null)
  (if (not (> _output_get 0.0))
    (bind _outactors (`GameplayStatics.GetAllActorsOfClass` "/Game/Blueprints/FPSController.FPSController_C"))
    (bind _asfpscontroller (cast `/Game/Blueprints/FPSController` (`|GetArrayItem` _outactors)))
    (set `/Game/Blueprints/FPSController.unlockedThree` true _asfpscontroller)
    (`self.K2_DestroyActor`)))

(fn `UserConstructionScript`)