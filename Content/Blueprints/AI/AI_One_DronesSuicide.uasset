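; Suicide drone AI actor that destroys itself on contact with the FPSController player or when shot down.
; A capsule hit from the player plays an impact sound and destroys the drone, with no damage dealt here.
; ProjectileTypeOne overlaps play the same sound and subtract projectile damage from AiHealth, destroying the drone at zero or below.
; Each overlap removes the first projectile found by GetAllActorsOfClass, not necessarily the overlapping one.
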(event `self.CapsuleComponent.OnComponentHit`
  (params (HitComponent :type "PrimitiveComponent Object Reference") (OtherActor :type "Actor Object Reference") (OtherComp :type "PrimitiveComponent Object Reference") (NormalImpulse :type "Vector Structure") (Hit :type "HitResult Structure (by ref)"))
  (cast `/Game/Blueprints/FPSController` OtherActor)
  (`GameplayStatics.PlaySoundAtLocation` "/Game/Sounds/projectilehit.projectilehit" (`SceneComponent.K2_GetComponentLocation` (`self.AIMesh`)) (struct) 1.0 1.0 0.0 null null null)
  (`self.K2_DestroyActor` :!label _label))

(event `self.CapsuleComponent.OnComponentBeginOverlap`
  (params (OverlappedComponent :type "PrimitiveComponent Object Reference") (OtherActor :type "Actor Object Reference") (OtherComp :type "PrimitiveComponent Object Reference") (OtherBodyIndex :type Integer) (bFromSweep :type Boolean) (SweepResult :type "HitResult Structure (by ref)"))
  (bind _asprojectile_type_one (cast `/Game/Blueprints/ProjectileTypeOne` OtherActor))
  (`GameplayStatics.PlaySoundAtLocation` "/Game/Sounds/projectilehit.projectilehit" (`SceneComponent.K2_GetComponentLocation` (`self.AIMesh`)) (struct) 1.0 1.0 0.0 null null null)
  (bind _output_get (set `self.aiHealth` (- (`self.aiHealth`) (`/Game/Blueprints/ProjectileTypeOne.projectileDamageValue` _asprojectile_type_one))))
  (bind _outactors (`GameplayStatics.GetAllActorsOfClass` "/Game/Blueprints/ProjectileTypeOne.ProjectileTypeOne_C"))
  (bind _asprojectile_type_one_2 (cast `/Game/Blueprints/ProjectileTypeOne` (`|GetArrayItem` _outactors)))
  (`self.K2_DestroyActor` _asprojectile_type_one_2)
  (if (not (> _output_get 0.0))
    (goto _label)))

(fn `UserConstructionScript`)