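; An AI enemy that fires AI_ProjectileThree at the player and can be destroyed by ProjectileTypeOne shots.
; Each tick it aims the spawn point at the first FPSController's Tracker; Detector overlaps toggle DetectedPlayer, which enables firing paced by a Delay on Tick.
; ProjectileTypeOne overlaps on Collision play a sound and subtract health, destroying the enemy at zero or below, while blocking hits destroy the projectile.
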(event `self.Collision.OnComponentHit`
  (params (HitComponent :type "PrimitiveComponent Object Reference") (OtherActor :type "Actor Object Reference") (OtherComp :type "PrimitiveComponent Object Reference") (NormalImpulse :type "Vector Structure") (Hit :type "HitResult Structure (by ref)"))
  (bind _asprojectile_type_one (cast `/Game/Blueprints/ProjectileTypeOne` OtherActor))
  (`self.K2_DestroyActor` _asprojectile_type_one))

(event `self.Collision.OnComponentBeginOverlap`
  (params (OverlappedComponent :type "PrimitiveComponent Object Reference") (OtherActor :type "Actor Object Reference") (OtherComp :type "PrimitiveComponent Object Reference") (OtherBodyIndex :type Integer) (bFromSweep :type Boolean) (SweepResult :type "HitResult Structure (by ref)"))
  (bind _asprojectile_type_one (cast `/Game/Blueprints/ProjectileTypeOne` OtherActor))
  (`GameplayStatics.PlaySoundAtLocation` "/Game/Sounds/projectilehit.projectilehit" (`SceneComponent.K2_GetComponentLocation` (`self.Cube`)) (struct) 1.0 1.0 0.0 null null null)
  (bind _output_get (set `self.aiHealth` (- (`self.aiHealth`) (`/Game/Blueprints/ProjectileTypeOne.projectileDamageValue` _asprojectile_type_one))))
  (if (not (> _output_get 0.0))
    (`self.K2_DestroyActor`)))

(event `self.ReceiveTick`
  (params (DeltaSeconds :type "Float (single-precision)"))
  (bind _projectilespawnpoint (`self.ProjectileSpawnPoint`))
  (bind _outactors (`GameplayStatics.GetAllActorsOfClass` "/Game/Blueprints/FPSController.FPSController_C"))
  (bind _asfpscontroller (cast `/Game/Blueprints/FPSController` (`|GetArrayItem` _outactors)))
  (`SceneComponent.K2_SetWorldRotation` (`self.ProjectileSpawnPoint`) (`KismetMathLibrary.FindLookAtRotation` (`SceneComponent.K2_GetComponentLocation` (`self.ProjectileSpawnPoint`)) (`SceneComponent.K2_GetComponentLocation` (`/Game/Blueprints/FPSController.Tracker` _asfpscontroller))) false false)
  (if (`self.detectedPlayer`)
    (`KismetSystemLibrary.Delay` 0.2)
    (`|SpawnActorFromClass` "/Game/Blueprints/AI/AI_ProjectileThree.AI_ProjectileThree_C" (`KismetMathLibrary.MakeTransform` (`SceneComponent.K2_GetComponentLocation` _projectilespawnpoint) (`SceneComponent.K2_GetComponentRotation` _projectilespawnpoint)) "Undefined" "OverrideRootScale" null null)))

(event `self.Detector.OnComponentBeginOverlap`
  (params (OverlappedComponent :type "PrimitiveComponent Object Reference") (OtherActor :type "Actor Object Reference") (OtherComp :type "PrimitiveComponent Object Reference") (OtherBodyIndex :type Integer) (bFromSweep :type Boolean) (SweepResult :type "HitResult Structure (by ref)"))
  (cast `/Game/Blueprints/FPSController` OtherActor)
  (set `self.detectedPlayer` true))

(event `self.Detector.OnComponentEndOverlap`
  (params (OverlappedComponent :type "PrimitiveComponent Object Reference") (OtherActor :type "Actor Object Reference") (OtherComp :type "PrimitiveComponent Object Reference") (OtherBodyIndex :type Integer))
  (cast `/Game/Blueprints/FPSController` OtherActor)
  (set `self.detectedPlayer` false))

(fn `UserConstructionScript`)