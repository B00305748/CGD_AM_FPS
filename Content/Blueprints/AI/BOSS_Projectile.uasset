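; Boss projectile actor that homes in on the player and damages them on contact.
; Every tick it finds the first FPSController, sets its Tracker component as the ProjectileMovement homing target, and copies the root component's tags onto Tags.
; When its collision component overlaps an FPSController, it subtracts ProjectileDamageValue directly from PlayerHealth and destroys itself, ignoring other actors.
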(event `self.ReceiveTick`
  (params (DeltaSeconds :type "Float (single-precision)"))
  (bind _outactors (`GameplayStatics.GetAllActorsOfClass` "/Game/Blueprints/FPSController.FPSController_C"))
  (bind _asfpscontroller (cast `/Game/Blueprints/FPSController` (`|GetArrayItem` _outactors)))
  (set `ProjectileMovementComponent.HomingTargetComponent` (`/Game/Blueprints/FPSController.Tracker` _asfpscontroller) (`self.ProjectileMovement`))
  (set `self.Tags` (`ActorComponent.ComponentTags` (`self.DefaultSceneRoot`))))

(event `self.projectileCollision.OnComponentBeginOverlap`
  (params (OverlappedComponent :type "PrimitiveComponent Object Reference") (OtherActor :type "Actor Object Reference") (OtherComp :type "PrimitiveComponent Object Reference") (OtherBodyIndex :type Integer) (bFromSweep :type Boolean) (SweepResult :type "HitResult Structure (by ref)"))
  (bind _asfpscontroller (cast `/Game/Blueprints/FPSController` OtherActor))
  (set `/Game/Blueprints/FPSController.playerHealth` (- (`/Game/Blueprints/FPSController.playerHealth` _asfpscontroller) (`self.projectileDamageValue`)) _asfpscontroller)
  (`self.K2_DestroyActor`))

(fn `UserConstructionScript`)