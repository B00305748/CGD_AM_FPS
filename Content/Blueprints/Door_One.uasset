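; Door_One is a sliding door Blueprint that opens when something overlaps its Box trigger and closes when the overlap ends.
; BeginPlay caches the world locations of the Start and End components.
; A Timeline plays forward or in reverse on overlap begin and end, lerping the Door component between those two locations.
; Any actor can trigger it, as the overlap events do not filter.
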(event `self.Box.OnComponentBeginOverlap`
  (params (OverlappedComponent :type "PrimitiveComponent Object Reference") (OtherActor :type "Actor Object Reference") (OtherComp :type "PrimitiveComponent Object Reference") (OtherBodyIndex :type Integer) (bFromSweep :type Boolean) (SweepResult :type "HitResult Structure (by ref)"))
  (bind (_direction _newtrack_0) (`Timeline|Timeline_0` :!label _label)
    (:`Update`
      (`SceneComponent.K2_SetWorldLocation` (`self.Door`) (`KismetMathLibrary.VLerp` (`self.WorldLocStart`) (`self.WorldLocEnd`) _newtrack_0) false false))))

(event `self.Box.OnComponentEndOverlap`
  (params (OverlappedComponent :type "PrimitiveComponent Object Reference") (OtherActor :type "Actor Object Reference") (OtherComp :type "PrimitiveComponent Object Reference") (OtherBodyIndex :type Integer))
  (goto _label :!via `Reverse`))

(event `self.ReceiveBeginPlay`
  (set `self.WorldLocStart` (`SceneComponent.K2_GetComponentLocation` (`self.Start`)))
  (set `self.WorldLocEnd` (`SceneComponent.K2_GetComponentLocation` (`self.End`))))

(fn `UserConstructionScript`)