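; LevelTwoKeyUnlocker is a damageable key actor that unlocks the level two door blocker when shot down.
; Overlaps from ProjectileTypeThree play an objective-complete sound and subtract projectile damage from KeyHealth.
; At depleted health, it destroys the first ProjectileTypeThree found, clears IsLocked on the first LevelTwoDoorBlocker and destroys itself.
; Targets come from GetAllActorsOfClass lookups, so the destroyed projectile may differ from the overlapping one.
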(event `self.Collision.OnComponentBeginOverlap`
  (params (OverlappedComponent :type "PrimitiveComponent Object Reference") (OtherActor :type "Actor Object Reference") (OtherComp :type "PrimitiveComponent Object Reference") (OtherBodyIndex :type Integer) (bFromSweep :type Boolean) (SweepResult :type "HitResult Structure (by ref)"))
  (bind _asprojectile_type_three (cast `/Game/Blueprints/ProjectileTypeThree` OtherActor))
  (`GameplayStatics.PlaySoundAtLocation` "/Game/Sounds/objectivecomplete.objectivecomplete" (`SceneComponent.K2_GetComponentLocation` (`self.Cube`)) (struct) 1.0 1.0 0.0 null null null)
  (bind _output_get (set `self.keyHealth` (- (`self.keyHealth`) (`/Game/Blueprints/ProjectileTypeThree.projectileDamageValue` _asprojectile_type_three))))
  (if (not (> _output_get 0.0))
    (bind _outactors (`GameplayStatics.GetAllActorsOfClass` "/Game/Blueprints/ProjectileTypeThree.ProjectileTypeThree_C"))
    (bind _asprojectile_type_three_2 (cast `/Game/Blueprints/ProjectileTypeThree` (`|GetArrayItem` _outactors)))
    (`self.K2_DestroyActor` _asprojectile_type_three_2)
    (bind _outactors_2 (`GameplayStatics.GetAllActorsOfClass` "/Game/Blueprints/Doorblockers/LevelTwoDoorBlocker.LevelTwoDoorBlocker_C"))
    (cast `/Game/Blueprints/Doorblockers/LevelTwoDoorBlocker` (`|GetArrayItem` _outactors_2))
    (`self.K2_DestroyActor`)
    (bind _outactors_3 (`GameplayStatics.GetAllActorsOfClass` "/Game/Blueprints/Doorblockers/LevelTwoDoorBlocker.LevelTwoDoorBlocker_C"))
    (set `/Game/Blueprints/Doorblockers/LevelTwoDoorBlocker.isLocked` false (`|GetArrayItem` _outactors_3))
    (`self.K2_DestroyActor`)))

(fn `UserConstructionScript`)