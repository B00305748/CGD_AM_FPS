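; Trigger actor that sends the player back to the level spawn and refills their health.
; When an FPSController overlaps EntranceCollision, its health and health gen packs are reset to their maximums.
; It then moves the player's root to the first SpawnLocationPoint found in the world, without sweeping, and plays the Health sound at the world origin.
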(event `self.EntranceCollision.OnComponentBeginOverlap`
  (params (OverlappedComponent :type "PrimitiveComponent Object Reference") (OtherActor :type "Actor Object Reference") (OtherComp :type "PrimitiveComponent Object Reference") (OtherBodyIndex :type Integer) (bFromSweep :type Boolean) (SweepResult :type "HitResult Structure (by ref)"))
  (bind _asfpscontroller (cast `/Game/Blueprints/FPSController` OtherActor))
  (set `/Game/Blueprints/FPSController.playerHealth` (`/Game/Blueprints/FPSController.maxHealth` _asfpscontroller) _asfpscontroller)
  (set `/Game/Blueprints/FPSController.healthGenPacks` (`/Game/Blueprints/FPSController.maxHealthGenPacks` _asfpscontroller) _asfpscontroller)
  (bind _outactors (`GameplayStatics.GetAllActorsOfClass` "/Game/Blueprints/LevelNavs/SpawnLocationPoint.SpawnLocationPoint_C"))
  (bind _asspawn_location_point (cast `/Game/Blueprints/LevelNavs/SpawnLocationPoint` (`|GetArrayItem` _outactors)))
  (`SceneComponent.K2_SetWorldLocation` (`Actor.RootComponent` _asfpscontroller) (`SceneComponent.K2_GetComponentLocation` (`Actor.RootComponent` _asspawn_location_point)) false false)
  (`GameplayStatics.PlaySoundAtLocation` "/Game/Sounds/health.health" (0.0 0.0 0.0) (struct) 1.0 1.0 0.0 null null null))

(fn `UserConstructionScript`)